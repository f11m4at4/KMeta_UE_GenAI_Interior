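; BP_Player is the shooting game's player, which moves on axis input and fires bullets.
; Horizontal and Vertical axis events share one setter that writes Direction's Y and Z, keeping X at zero.
; Tick moves the actor by Direction, Speed and delta time, without sweep.
; Pressing Fire spawns a BP_Bullet at the FirePosition component's world location and plays a blaster sound.
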(event `self.ReceiveBeginPlay`
  (`KismetSystemLibrary.PrintString` "Hello World"))

(event `self.ReceiveTick`
  (params (DeltaSeconds :type "Float (single-precision)"))
  ; 이동한다.
  (`self.K2_SetActorLocation` (+ (* DeltaSeconds (* (`self.Direction`) (`self.Speed`))) (`self.K2_GetActorLocation`))))

(event `InputAxis|Horizontal`
  (params (AxisValue :type "Float (single-precision)"))
  ; 방향구하기
  (set `self.Direction` (`KismetMathLibrary.MakeVector` 0.0 AxisValue (stale `InputAxis|Vertical` AxisValue)) :!label _label))

(event `InputAxis|Vertical`
  (params (AxisValue :type "Float (single-precision)"))
  ; 방향구하기
  (goto _label))

(event `InputAction|Fire`
  (params (Key :type "Key Structure"))
  (:`Pressed`
    (`|SpawnActorFromClass` "/Game/Shooting/Blueprints/BP_Bullet.BP_Bullet_C" (`KismetMathLibrary.MakeTransform` (`SceneComponent.K2_GetComponentLocation` (`self.FirePosition`))) "Undefined" "MultiplyWithRoot" null null)
    (`GameplayStatics.PlaySound2D` "/Game/Shooting/star-wars-blaster.star-wars-blaster" 1.0 1.0 0.0 null null)))

(fn `UserConstructionScript`)