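; BP_Enemy is a shooting-game enemy that homes in on the player and explodes on contact.
; On BeginPlay it caches the BP_Player actor as its target.
; Each Tick it moves straight toward the target's current position at Speed, scaled by delta time and without sweep.
; Any overlap with its Body destroys both the other actor and itself, then spawns an explosion effect and plays a bomb sound.
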(event `self.ReceiveBeginPlay`
  (bind _returnvalue (`GameplayStatics.GetActorOfClass` "/Game/Shooting/Blueprints/BP_Player.BP_Player_C"))
  (set `self.Target` _returnvalue))

(event `self.ReceiveTick`
  (params (DeltaSeconds :type "Float (single-precision)"))
  ; 이동한다.
  (set `self.Direction` (`KismetMathLibrary.Normal` (- (`self.K2_GetActorLocation` (`self.Target`)) (`self.K2_GetActorLocation`))))
  (`self.K2_SetActorLocation` (+ (* DeltaSeconds (* (`self.Direction`) (`self.Speed`))) (`self.K2_GetActorLocation`))))

(event `self.Body.OnComponentBeginOverlap`
  (params (OverlappedComponent :type "PrimitiveComponent Object Reference") (OtherActor :type "Actor Object Reference") (OtherComp :type "PrimitiveComponent Object Reference") (OtherBodyIndex :type Integer) (bFromSweep :type Boolean) (SweepResult :type "HitResult Structure (by ref)"))
  (`self.K2_DestroyActor` OtherActor)
  (`self.K2_DestroyActor`)
  (`GameplayStatics.SpawnEmitterAtLocation` "/Game/StarterContent/Particles/P_Explosion.P_Explosion" (`self.K2_GetActorLocation`))
  (`GameplayStatics.PlaySound2D` "/Game/Shooting/BombSound.BombSound" 1.0 1.0 0.0 null null))

(fn `UserConstructionScript`)