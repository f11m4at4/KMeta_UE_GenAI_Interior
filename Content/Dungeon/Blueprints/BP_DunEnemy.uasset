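; Dungeon enemy Blueprint that finds the BP_DunPlayer on BeginPlay and chases it with AI MoveToActor.
; A Tick-driven enum state machine waits in Idle, switches to Move, then enters Attack once the player is within range.
; Delay nodes time the Idle exit and repeat the attack, which only prints a message and never returns to Move.
; Damage and Die are empty stubs, and the current state prints every tick.
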(event `MoveToTarget`
  (bind _targetplayer (`self.TargetPlayer`))
  ; 이동
  ;; Target 이 있을때만처리
  (`/Engine/EditorBlueprintResources/StandardMacros.IsValid` _targetplayer
    (:`Is Valid`
      (`AIController.MoveToActor` (`AIBlueprintHelperLibrary.GetAIController` (`self.GetController`)) _targetplayer -1.0 true true true null true))))

(event `self.ReceiveBeginPlay`
  ; 태어날때 타겟찾기
  (bind _returnvalue (`GameplayStatics.GetActorOfClass` "/Game/Dungeon/Blueprints/BP_DunPlayer.BP_DunPlayer_C"))
  (set `self.TargetPlayer` _returnvalue))

(event `self.ReceiveTick`
  (params (DeltaSeconds :type "Float (single-precision)"))
  ; 살아가는 동안 행동할 목차 설정
  (`KismetSystemLibrary.PrintString` (`|GetEnumeratorNameAsString` (`self.CurState`)))
  (switch `/Game/Dungeon/Blueprints/EEnemyState` (`self.CurState`)
    (:`NewEnumerator0`
      (`self.IdleState`))
    (:`NewEnumerator1`
      (`self.MoveState`))
    (:`NewEnumerator2`
      (`self.AttackState`))
    (:`NewEnumerator3`
      (`self.DamageState`))
    (:`NewEnumerator4`
      (`self.DieState`))))

(event `IdleState`
  ; 일정시간이 지나면 상태를 이동으로 전환하고 싶다.
  (`KismetSystemLibrary.Delay` (`self.IdleDelayTime`))
  (set `self.CurState` "NewEnumerator1"))

(event `MoveState`
  ; 이동상태
  (`self.MoveToTarget`)
  (if (< (`KismetMathLibrary.Vector_Distance` (`self.K2_GetActorLocation`) (`self.K2_GetActorLocation` (`self.TargetPlayer`))) (`self.AttackRange`))
    (set `self.CurState` "NewEnumerator2")))

(event `AttackState`
  ; 일정시간에한번씩공격하기
  (`KismetSystemLibrary.Delay` (`self.AttackDelayTime`))
  (`KismetSystemLibrary.PrintString` "공격!!!"))

(event `DamageState`)

(event `DieState`)

(fn `UserConstructionScript`)