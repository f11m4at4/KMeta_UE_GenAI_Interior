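; BP_DunPlayer is the player Character for the Dungeon game, handling movement, camera look, jumping and running through Enhanced Input.
; BeginPlay adds the IMC_Dungeon mapping context to the first player controller's input subsystem.
; Move actions follow the right and forward vectors of the full control rotation, which the look actions drive through yaw and pitch.
; Holding Run raises CharacterMovement's max walk speed until release.
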(event `self.ReceiveBeginPlay`
  (`EnhancedInputSubsystemInterface.AddMappingContext` (pcsubsystem `EnhancedInputLocalPlayerSubsystem` (`GameplayStatics.GetPlayerController` 0)) "/Game/Dungeon/Inputs/IMC_Dungeon.IMC_Dungeon" 0 (struct)))

(event `EnhancedInput|/Game/Dungeon/Inputs/IA_Horizontal`
  (params (ActionValue :type "Float (double-precision)") (ElapsedSeconds :type "Float (double-precision)") (TriggeredSeconds :type "Float (double-precision)") (InputAction :type "InputAction Object Reference" :default "/Game/Dungeon/Inputs/IA_Horizontal.IA_Horizontal"))
  ; 이동
  (:`Triggered`
    (`self.AddMovementInput` (`KismetMathLibrary.GetRightVector` (`self.GetControlRotation`)) ActionValue)))

(event `EnhancedInput|/Game/Dungeon/Inputs/IA_Vertical`
  (params (ActionValue :type "Float (double-precision)") (ElapsedSeconds :type "Float (double-precision)") (TriggeredSeconds :type "Float (double-precision)") (InputAction :type "InputAction Object Reference" :default "/Game/Dungeon/Inputs/IA_Vertical.IA_Vertical"))
  ; 이동
  (:`Triggered`
    (`self.AddMovementInput` (`KismetMathLibrary.GetForwardVector` (`self.GetControlRotation`)) ActionValue)))

(event `EnhancedInput|/Game/Dungeon/Inputs/IA_CamTurn`
  (params (ActionValue :type "Float (double-precision)") (ElapsedSeconds :type "Float (double-precision)") (TriggeredSeconds :type "Float (double-precision)") (InputAction :type "InputAction Object Reference" :default "/Game/Dungeon/Inputs/IA_CamTurn.IA_CamTurn"))
  ; 회전
  (:`Triggered`
    (`self.AddControllerYawInput` ActionValue)))

(event `EnhancedInput|/Game/Dungeon/Inputs/IA_CamLookup`
  (params (ActionValue :type "Float (double-precision)") (ElapsedSeconds :type "Float (double-precision)") (TriggeredSeconds :type "Float (double-precision)") (InputAction :type "InputAction Object Reference" :default "/Game/Dungeon/Inputs/IA_CamLookup.IA_CamLookup"))
  ; 회전
  (:`Triggered`
    (`self.AddControllerPitchInput` ActionValue)))

(event `EnhancedInput|/Game/Dungeon/Inputs/IA_PlayerJump`
  (params (ActionValue :type Boolean) (ElapsedSeconds :type "Float (double-precision)") (TriggeredSeconds :type "Float (double-precision)") (InputAction :type "InputAction Object Reference" :default "/Game/Dungeon/Inputs/IA_PlayerJump.IA_PlayerJump"))
  (:`Started`
    (`self.Jump`)))

(event `EnhancedInput|/Game/Dungeon/Inputs/IA_Run`
  (params (ActionValue :type Boolean) (ElapsedSeconds :type "Float (double-precision)") (TriggeredSeconds :type "Float (double-precision)") (InputAction :type "InputAction Object Reference" :default "/Game/Dungeon/Inputs/IA_Run.IA_Run"))
  (bind _charactermovement (`self.CharacterMovement`))
  (:`Started`
    (set `CharacterMovementComponent.MaxWalkSpeed` 600.0 _charactermovement))
  (:`Completed`
    (set `CharacterMovementComponent.MaxWalkSpeed` 200.0 _charactermovement)))

(fn `UserConstructionScript`)